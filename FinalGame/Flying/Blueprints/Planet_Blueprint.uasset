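; Planet actor for the flying game that counts hits and ends the game on the second one.
; Each hit, after a short delay, deactivates the Fire component, plays an explosion sound and increments NumHits.
; Tick polls that counter and, when it equals two, pauses the game, adds a GameOver widget to the viewport and shows the mouse cursor.
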(event EventTick
  (params (DeltaSeconds :type Float%20%28single-precision%29))
  ;[1 1 1] Add 1 to Number of Hits - 2 hits = game over
  (if (== 2 (Variables|Default|GetNumHits))
    (Game|SetGamePaused true)
    (bind _returnvalue (UserInterface|CreateWidget "/Game/UMG/GameOver.GameOver_C"))
    (UserInterface|Viewport|AddtoViewport _returnvalue 0)
    (Variables|/Script/Engine.PlayerController|SetbShowMouseCursor (Game|GetPlayerController 0) true)))

(event Collision|EventHit
  (params (MyComp :type Primitive%20Component%20Object%20Reference) (Other :type Actor%20Object%20Reference) (OtherComp :type Primitive%20Component%20Object%20Reference) (bSelfMoved :type Boolean) (HitLocation :type Vector :default "0, 0, 0") (HitNormal :type Vector :default "0, 0, 0") (NormalImpulse :type Vector :default "0, 0, 0") (Hit :type Hit%20Result%20Structure%20%28by%20ref%29))
  ;[1 1 1] On hit planet - play explosion effect
  (Utilities|FlowControl|Delay 0.2)
  (Components|Activation|SetActive (Variables|Default|GetFire) false false)
  (Audio|PlaySoundatLocation "/Game/StarterContent/Audio/Explosion01.Explosion01" "0, 0, 0")
  (Variables|Default|SetNumHits (+ 1 (Variables|Default|GetNumHits))))

(fn ConstructionScript)